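; Player stats component that tracks current and max health and stamina for its owning BP_ThirdPersonCharacter.
; One tick after BeginPlay it caches the character and fills both HUD bars.
; Increase and decrease functions change the values and push them straight to the HUD bars, plus the health text for health.
; Decrease functions return true once the stat is depleted, and increases to current values cap at the maximum.
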(event `self.ReceiveBeginPlay`
  (`KismetSystemLibrary.DelayUntilNextTick`)
  (bind _asbp_third_person_character (cast `/Game/ThirdPerson/Blueprints/BP_ThirdPersonCharacter` (`self.GetOwner`)))
  (set `self.PlayerCharacterBP` _asbp_third_person_character)
  (`ProgressBar.SetPercent` (`/Game/UI/WB_HUD.StaminaBar` (`/Game/ThirdPerson/Blueprints/BP_ThirdPersonCharacter.HUDWidgget` (`self.PlayerCharacterBP`))) (/ (`self.CurrentStamina`) (`self.MaxStamina`)))
  (`ProgressBar.SetPercent` (`/Game/UI/WB_HUD.HealthBar` (`/Game/ThirdPerson/Blueprints/BP_ThirdPersonCharacter.HUDWidgget` (`self.PlayerCharacterBP`))) (/ (`self.CurrentHealth`) (`self.MaxHealth`))))

(fn `DecreaseHealth`
  (params (HealthDamage :type "Float (double-precision)"))
  (returns (IsPlayerDead :type Boolean))
  (bind _hudwidgget (`/Game/ThirdPerson/Blueprints/BP_ThirdPersonCharacter.HUDWidgget` (`self.PlayerCharacterBP`)))
  (if (not (<= (`self.CurrentHealth`) 0.0))
    (bind _output_get (set `self.CurrentHealth` (- (`self.CurrentHealth`) HealthDamage)))
    (`ProgressBar.SetPercent` (`/Game/UI/WB_HUD.HealthBar` _hudwidgget) (/ _output_get (`self.MaxHealth`)))
    (`TextBlock.SetText` (`/Game/UI/WB_HUD.HealthText` _hudwidgget) (`KismetTextLibrary.Conv_DoubleToText` (`self.CurrentHealth`) "HalfToEven"))
    (if (<= (`self.CurrentHealth`) 0.0)
      _
      (else
        (return false))))
  (return true))

(fn `DecreaseStamina`
  (params (StaminaDamage :type "Float (double-precision)"))
  (returns (NoStaminaLeft :type Boolean))
  (if (not (<= (`self.CurrentStamina`) 0.0))
    (set `self.CurrentStamina` (- (`self.CurrentStamina`) StaminaDamage))
    (`ProgressBar.SetPercent` (`/Game/UI/WB_HUD.StaminaBar` (`/Game/ThirdPerson/Blueprints/BP_ThirdPersonCharacter.HUDWidgget` (`self.PlayerCharacterBP`))) (/ (`self.CurrentStamina`) (`self.MaxStamina`)))
    (if (<= (`self.CurrentStamina`) 0.0)
      _
      (else
        (return false))))
  (return true))

(fn `IncreaseHealth`
  (params (HealthIncrease :type "Float (double-precision)"))
  (bind _hudwidgget (`/Game/ThirdPerson/Blueprints/BP_ThirdPersonCharacter.HUDWidgget` (`self.PlayerCharacterBP`)))
  (set `self.CurrentHealth` (+ (`self.CurrentHealth`) HealthIncrease))
  (if (> (`self.CurrentHealth`) (`self.MaxHealth`))
    (set `self.CurrentHealth` (`self.MaxHealth`)))
  (`ProgressBar.SetPercent` (`/Game/UI/WB_HUD.HealthBar` _hudwidgget) (/ (`self.CurrentHealth`) (`self.MaxHealth`)))
  (`TextBlock.SetText` (`/Game/UI/WB_HUD.HealthText` _hudwidgget) (`KismetTextLibrary.Conv_DoubleToText` (`self.CurrentHealth`) "HalfToEven")))

(fn `IncreaseMaxHealth`
  (params (MaxHealthIncrease :type "Float (double-precision)"))
  (bind _hudwidgget (`/Game/ThirdPerson/Blueprints/BP_ThirdPersonCharacter.HUDWidgget` (`self.PlayerCharacterBP`)))
  (set `self.MaxHealth` (+ (`self.MaxHealth`) MaxHealthIncrease))
  (`ProgressBar.SetPercent` (`/Game/UI/WB_HUD.HealthBar` _hudwidgget) (/ (`self.CurrentHealth`) (`self.MaxHealth`)))
  (`TextBlock.SetText` (`/Game/UI/WB_HUD.HealthText` _hudwidgget) (`KismetTextLibrary.Conv_DoubleToText` (`self.CurrentHealth`) "HalfToEven")))

(fn `IncreaseMaxStamina`
  (params (StaminaMaxIncrease :type "Float (double-precision)"))
  (set `self.MaxStamina` (+ (`self.MaxStamina`) StaminaMaxIncrease))
  (`ProgressBar.SetPercent` (`/Game/UI/WB_HUD.StaminaBar` (`/Game/ThirdPerson/Blueprints/BP_ThirdPersonCharacter.HUDWidgget` (`self.PlayerCharacterBP`))) (/ (`self.CurrentStamina`) (`self.MaxStamina`))))

(fn `IncreaseStamina`
  (params (StaminaIncrease :type "Float (double-precision)"))
  (set `self.CurrentStamina` (+ (`self.CurrentStamina`) StaminaIncrease))
  (if (> (`self.CurrentStamina`) (`self.MaxStamina`))
    (set `self.CurrentStamina` (`self.MaxStamina`)))
  (`ProgressBar.SetPercent` (`/Game/UI/WB_HUD.StaminaBar` (`/Game/ThirdPerson/Blueprints/BP_ThirdPersonCharacter.HUDWidgget` (`self.PlayerCharacterBP`))) (/ (`self.CurrentStamina`) (`self.MaxStamina`))))